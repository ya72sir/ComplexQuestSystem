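; NPC Blueprint for a quest giver who offers a quest once the player has enough prestige in a required region.
; When the player's regional prestige meets the requirement, the NPC becomes able to give the quest and shows its question mark.
; On interaction it adds and immediately starts the quest through the character's quest manager, hides the marker and changes its default message.
; Otherwise, interaction falls through to the parent NPC behavior.
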(event `self.OnInteractWith`
  (params (Character :type "/Game/QuestSystem/Blueprints/Characters/ThirdPersonCharacter Object Reference"))
  (if (and (`self.CanGiveQuest?`) (not (`self.HasGivenQuest?`)))
    (`/Game/QuestSystem/Blueprints/Actors/BP_QuestManager.-AddNewQuest` (`/Game/QuestSystem/Blueprints/Characters/ThirdPersonCharacter.QuestManagerRef` Character) (`self.QuestToGive`) true)
    (set `self.HasGivenQuest?` true)
    (set `self.DefaultMessage` "You have finally become an honourable and respected man! ")
    (`SceneComponent.SetVisibility` (`self.QuestionMark`) false false)
    (else
      (`parent.OnInteractWith` Character))))

(event `self.OnPlayerGainPrestige`
  (params (Player :type "/Game/QuestSystem/Blueprints/Characters/ThirdPersonCharacter Object Reference"))
  (bind (_region _prestige) (break `/Game/QuestSystem/Blueprints/Structures/s_RegionPrestige` (`self.RequiredPrestige`)))
  (if (and (>= (`/Game/QuestSystem/Blueprints/Characters/ThirdPersonCharacter.-GetPrestigeByRegion` Player _region) _prestige) (not (`self.CanGiveQuest?`)) (not (`self.HasGivenQuest?`)))
    (set `self.CanGiveQuest?` true)
    (`SceneComponent.SetVisibility` (`self.QuestionMark`) true false)))

(fn `UserConstructionScript`
  (`parent.UserConstructionScript`))