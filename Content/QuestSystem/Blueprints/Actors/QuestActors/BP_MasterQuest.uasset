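; BP_MasterQuest is a quest actor that tracks active and completed sub-goals, hunt counts and the running quest description.
; Completing a sub-goal fires the empty OnGoalCompleted event, adds its following goals and updates the quest widget and journal.
; AddGoalForIndex creates goal widgets, or recursively auto-completes goals whose target object the player already obtained.
; GoToNextSubGoal offers linear advancement by index alongside this branching flow.
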(event `OnGoalCompleted`
  (params (GoalIndex :type Integer)))

(fn `-AddGoalForIndex`
  (params (Index :type Integer))
  (locals (localIndex :type Integer))
  (bind _questwidget (`self.QuestWidget`))
  (bind _localindex (`local.localIndex`))
  (bind _goal (`self.-GoalAtIndex` (`local.localIndex`)))
  (bind _goal_2 (`self.-GoalAtIndex` _localindex))
  (bind _output_get (set `local.localIndex` Index))
  (if (`self.-GoalAlreadyFound?` _output_get)
    (`KismetArrayLibrary.Array_Add` (`self.CompletedSubGoals`) (make `/Game/QuestSystem/Blueprints/Structures/s_CompletedGoal` _localindex _goal_2 true))
    (`self.OnGoalCompleted` (`local.localIndex`))
    (for _array_element (`.FollowingSubGoalIndices_26_17B2172546AD70BC6309B0BA371DB121` (break `/Game/QuestSystem/Blueprints/Structures/s_GoalInfo` _goal_2))
      (`self.-AddGoalForIndex` _array_element))
    (return)
    (else
      (bind _returnvalue (`KismetArrayLibrary.Array_Add` (`self.CurrentGoalIndices`) (`local.localIndex`)))
      (if (> _returnvalue (`KismetArrayLibrary.Array_LastIndex` (`self.CurrentHuntedAmounts`)))
        (`KismetArrayLibrary.Array_Add` (`self.CurrentHuntedAmounts`)))
      (`KismetArrayLibrary.Array_Add` (`self.CurrentGoal`) _goal)
      (bind _returnvalue_2 (`|CreateWidget` "/Game/QuestSystem/Widgets/w_SubGoalWidget.w_SubGoalWidget_C" null _goal self (`self.QuestWidget`)))
      (`KismetArrayLibrary.Array_Add` (`/Game/QuestSystem/Widgets/w_QuestWidget.SubGoalWidget` _questwidget) _returnvalue_2)
      (`PanelWidget.AddChild` (`/Game/QuestSystem/Widgets/w_QuestWidget.SubGoalBox` _questwidget) _returnvalue_2)
      (return))))

(fn `-CompleteSubGoal`
  (params (SubGoalIndex :type Integer))
  (returns (`Success?` :type Boolean))
  (locals (localGoalIndex :type Integer) (localCompletedGoal :type "/Game/QuestSystem/Blueprints/Structures/s_GoalInfo Structure") (localWidgetIndex :type Integer :default 0))
  (bind _questwidget (`self.QuestWidget`))
  (bind _currentgoalindices (`self.CurrentGoalIndices`))
  (bind ((`UpdateQuestDescription?_19_9983560E41A16B702BBF52855D493785` _updatequestdescription_) (`UpdateDescription_22_790B84114CE074E0277C328F9BD35BB6` _updatedescription)) (break `/Game/QuestSystem/Blueprints/Structures/s_GoalInfo` (`local.localCompletedGoal`)))
  (bind _returnvalue (`KismetArrayLibrary.Array_Find` _currentgoalindices (`local.localGoalIndex`)))
  (bind _subgoalwidget (`/Game/QuestSystem/Widgets/w_QuestWidget.SubGoalWidget` (`self.QuestWidget`)))
  (set `local.localGoalIndex` SubGoalIndex)
  (if (`KismetArrayLibrary.Array_Contains` (`self.CurrentGoalIndices`) (`local.localGoalIndex`))
    (bind _output_get (set `local.localCompletedGoal` (`|GetArrayItem` (`.SubGoals_28_013B6E9547A400FFB6191DA95AA944FF` (break `/Game/QuestSystem/Blueprints/Structures/s_QuestInfo` (`self.QuestInfo`))) (`local.localGoalIndex`))))
    (`KismetArrayLibrary.Array_Add` (`self.CompletedSubGoals`) (make `/Game/QuestSystem/Blueprints/Structures/s_CompletedGoal` (`local.localGoalIndex`) _output_get true))
    (if _updatequestdescription_
      (set `self.CurrentDescription` (`|FormatText` "{Current}{Next}" (`self.CurrentDescription`) _updatedescription))
      (if (`self.-SelectedInJournal?`)
        (`/Game/QuestSystem/Widgets/w_QuestJournal.-UpdateDescription` (`/Game/QuestSystem/Widgets/w_MainWidget.w_QuestJournal` (`/Game/QuestSystem/Blueprints/Actors/BP_QuestManager.MainWidget` (`self.QuestManager`))))))
    (`KismetArrayLibrary.Array_RemoveItem` (`self.CurrentGoal`) (`local.localCompletedGoal`))
    (set `local.localWidgetIndex` _returnvalue)
    (`KismetArrayLibrary.Array_Remove` (`self.CurrentHuntedAmounts`) _returnvalue)
    (`KismetArrayLibrary.Array_RemoveItem` _currentgoalindices (`local.localGoalIndex`))
    (`Widget.RemoveFromParent` (`|GetArrayItem` _subgoalwidget (`local.localWidgetIndex`)))
    (`KismetArrayLibrary.Array_Remove` _subgoalwidget (`local.localWidgetIndex`))
    (`self.OnGoalCompleted` (`local.localGoalIndex`))
    (for _array_element (`.FollowingSubGoalIndices_26_17B2172546AD70BC6309B0BA371DB121` (break `/Game/QuestSystem/Blueprints/Structures/s_GoalInfo` (`local.localCompletedGoal`)))
      (`self.-AddGoalForIndex` _array_element))
    (if (`self.-SelectedInJournal?`)
      (`/Game/QuestSystem/Widgets/w_QuestJournal.-GenerateSubGoals` (`/Game/QuestSystem/Widgets/w_MainWidget.w_QuestJournal` (`/Game/QuestSystem/Blueprints/Actors/BP_QuestManager.MainWidget` (`self.QuestManager`)))))
    (if (and (== (`local.localGoalIndex`) (`self.SelectedSubGoalIndex`)) (== (`/Game/QuestSystem/Blueprints/Actors/BP_QuestManager.CurrentQuest` (`self.QuestManager`)) self))
      (`/Game/QuestSystem/Widgets/w_QuestWidget.-SelectSubGoal` _questwidget (`|GetArrayItem` (`/Game/QuestSystem/Widgets/w_QuestWidget.SubGoalWidget` _questwidget)))
      (return true)
      (else
        (return true)))
    (else
      (return false))))

(fn `-GoalAlreadyFound?`
  (params (GoalIndex :type Integer))
  (returns (Out :type Boolean))
  (locals (localBool :type Boolean))
  (bind (_type _customgoal_ _goaltext _additionalname _amounttohunt _goalclass) (break `/Game/QuestSystem/Blueprints/Structures/s_GoalInfo` (`self.-GoalAtIndex` GoalIndex)))
  (if (`|EnumEquality` _type "NewEnumerator2")
    (for _array_element (`/Game/QuestSystem/Blueprints/Characters/ThirdPersonCharacter.ObtainedObject` (`/Game/QuestSystem/Blueprints/Actors/BP_QuestManager.ThirdPersonChar` (`self.QuestManager`)))
      (if (== _array_element _goalclass)
        (set `local.localBool` true)
        (break)))
    (return (`local.localBool`))
    (else
      (return false))))

(fn `-GoalAtIndex`
  (params (Index :type Integer))
  (returns (Goal :type "/Game/QuestSystem/Blueprints/Structures/s_GoalInfo Structure"))
  (return (`|GetArrayItem` (`.SubGoals_28_013B6E9547A400FFB6191DA95AA944FF` (break `/Game/QuestSystem/Blueprints/Structures/s_QuestInfo` (`self.QuestInfo`))) Index)))

(fn `-GoToNextSubGoal`
  (returns (`Success?` :type Boolean))
  (locals (L_NextIndex :type Integer :default 0))
  (bind _currentgoalindices (`self.CurrentGoalIndices`))
  (bind _returnvalue (+ (`.MaxValue` (`KismetMathLibrary.MaxOfIntArray` (`self.CurrentGoalIndices`))) 1))
  (if (<= _returnvalue (`KismetArrayLibrary.Array_Length` (`.SubGoals_28_013B6E9547A400FFB6191DA95AA944FF` (break `/Game/QuestSystem/Blueprints/Structures/s_QuestInfo` (`self.QuestInfo`)))))
    (set `local.L_NextIndex` _returnvalue)
    (`KismetArrayLibrary.Array_Clear` _currentgoalindices)
    (`KismetArrayLibrary.Array_Add` _currentgoalindices (`local.L_NextIndex`))
    (`self.-UpdateSubGoals`)
    (return true)
    (else
      (return false))))

(fn `-SelectedInJournal?`
  (returns (`Out?` :type Boolean))
  (bind _selectedquest (`/Game/QuestSystem/Widgets/w_QuestJournal.SelectedQuest` (`/Game/QuestSystem/Widgets/w_MainWidget.w_QuestJournal` (`/Game/QuestSystem/Blueprints/Actors/BP_QuestManager.MainWidget` (`self.QuestManager`)))))
  (return (and (== _selectedquest self) (`KismetSystemLibrary.IsValid` _selectedquest))))

(fn `-SetupStartingGoals`
  (`KismetArrayLibrary.Array_Clear` (`self.CurrentGoalIndices`))
  (for _array_element (`self.StartingSubGoalIndices`)
    (`self.-AddGoalForIndex` _array_element))
  (`KismetArrayLibrary.Array_Resize` (`self.CurrentHuntedAmounts`) (`KismetArrayLibrary.Array_Length` (`self.CurrentGoalIndices`)))
  (`self.-UpdateSubGoals`)
  (set `self.CurrentDescription` (`.Description_8_B762635B4A5A78AD320EF4B3582066E6` (break `/Game/QuestSystem/Blueprints/Structures/s_QuestInfo` (`self.QuestInfo`))))
  (return))

(fn `-UpdateSubGoals`
  (`KismetArrayLibrary.Array_Clear` (`self.CurrentGoal`))
  (for _array_element (`self.CurrentGoalIndices`)
    (`KismetArrayLibrary.Array_Add` (`self.CurrentGoal`) (`|GetArrayItem` (`.SubGoals_28_013B6E9547A400FFB6191DA95AA944FF` (break `/Game/QuestSystem/Blueprints/Structures/s_QuestInfo` (`self.QuestInfo`))) _array_element)))
  (return))

(fn `UserConstructionScript`)